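; BP_Button is a clickable world button that spawns a BP_Turtle each time it is clicked.
; The turtle spawns offset along world X from the button's Cube, with Start at that point, Target farther along X, and the button's Type passed through.
; Cursor-over events swap the Cube's material to red on hover and back to normal when the cursor leaves.
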(event MouseInput|EventActorOnClicked
  (params (ButtonPressed :type Key%20Structure :default "None"))
  (bind _cube (Variables|Components|GetCube))
  (bind _returnvalue (Transformation|GetWorldTransform _cube))
  (bind (_location _rotation _scale) (Math|Transform|BreakTransform _returnvalue))
  (bind (_x _y _z) (Math|Vector|BreakVector _location))
  (bind _returnvalue_2 (+ _x 4e+02))
  (bind _returnvalue_3 (Math|Vector|MakeVector _returnvalue_2 _y _z))
  (Game|SpawnActorfromClass "/Game/Characters/Turtle/BP_Turtle.BP_Turtle_C" (Math|Transform|MakeTransform _returnvalue_3 _rotation _scale) "AlwaysSpawn" 0 _returnvalue_3 (Math|Vector|MakeVector (+ _x 1e+03) _y _z) (Variables|Default|GetType) 0))

(event MouseInput|EventActorBeginCursorOver
  (Rendering|Material|SetMaterial (Variables|Components|GetCube) 0 "/Game/Matereials/ButtonRed.ButtonRed"))

(event MouseInput|EventActorEndCursorOver
  (Rendering|Material|SetMaterial (Variables|Components|GetCube) 0 "/Game/Matereials/ButtonNormal.ButtonNormal"))

(fn ConstructionScript)